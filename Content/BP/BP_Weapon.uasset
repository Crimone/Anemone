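; BP_Weapon is a weapon pickup actor that reacts when a ThirdPersonCharacter comes within its sphere.
; On overlap it shows the Tip widget, passes its Name to UI_WeaponPickUp, enables custom depth on the mesh and calls PickupOpen on the character with itself.
; Leaving the sphere hides the tip, disables custom depth and calls PickupClose.
; An IsRotation-driven mesh spin is present but disconnected, and Tick is empty.
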(event `self.ReceiveTick`
  (params (DeltaSeconds :type "Float (single-precision)")))

(event `self.Sphere.OnComponentBeginOverlap`
  (params (OverlappedComponent :type "PrimitiveComponent Object Reference") (OtherActor :type "Actor Object Reference") (OtherComp :type "PrimitiveComponent Object Reference") (OtherBodyIndex :type Integer) (bFromSweep :type Boolean) (SweepResult :type "HitResult Structure (by ref)"))
  (bind _asthird_person_character (cast `/Game/ThirdPersonBP/Blueprints/ThirdPersonCharacter` OtherActor))
  (`SceneComponent.SetVisibility` (`self.Tip`) true true)
  (`/Game/ThirdPersonBP/Blueprints/ThirdPersonCharacter.PickupOpen` _asthird_person_character self)
  (bind _asui_weapon_pick_up (cast `/Game/BP/UI_WeaponPickUp` (`WidgetComponent.GetWidget` (`self.Tip`))))
  (set `/Game/BP/UI_WeaponPickUp.Name` (`self.Name`) _asui_weapon_pick_up)
  (`PrimitiveComponent.SetRenderCustomDepth` (`self.SkeletalMesh`) true))

(event `self.Sphere.OnComponentEndOverlap`
  (params (OverlappedComponent :type "PrimitiveComponent Object Reference") (OtherActor :type "Actor Object Reference") (OtherComp :type "PrimitiveComponent Object Reference") (OtherBodyIndex :type Integer))
  (bind _asthird_person_character (cast `/Game/ThirdPersonBP/Blueprints/ThirdPersonCharacter` OtherActor))
  (`SceneComponent.SetVisibility` (`self.Tip`) false true)
  (`/Game/ThirdPersonBP/Blueprints/ThirdPersonCharacter.PickupClose` _asthird_person_character)
  (`PrimitiveComponent.SetRenderCustomDepth` (`self.SkeletalMesh`) false))

(fn `UserConstructionScript`)